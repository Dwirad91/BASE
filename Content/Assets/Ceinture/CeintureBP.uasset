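; CeintureBP is a belt pickup that attaches itself to a player who walks into its Box trigger.
; The overlap calls CeintureServeurEquip, which forwards to CeintureClientEquip, a server/client naming split.
; If the PlayerBase's Ceinture value is false or unset, the mesh collision is disabled and a component snaps to the CeintureSocket on the player's mesh.
; This graph never sets Ceinture, and the Sphere overlap events are empty.
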(event `CeintureClientEquip`
  (params (Object :type "Object Object Reference"))
  (bind _asplayer_base (cast `/Game/ThirdPersonBP/Blueprints/PlayerBase` Object))
  (if (not (`/Game/ThirdPersonBP/Blueprints/PlayerBase.Ceinture?` _asplayer_base))
    (`PrimitiveComponent.SetCollisionEnabled` (`self.SkeletalMesh`) "NoCollision")
    (`self.K2_AttachToComponent` (`Character.Mesh` _asplayer_base) "CeintureSocket" "SnapToTarget" "SnapToTarget" "SnapToTarget")))

(event `CeintureServeurEquip`
  (params (Object :type "Object Object Reference"))
  (`self.CeintureClientEquip` Object))

(event `self.Box.OnComponentBeginOverlap`
  (params (OverlappedComponent :type "PrimitiveComponent Object Reference") (OtherActor :type "Actor Object Reference") (OtherComp :type "PrimitiveComponent Object Reference") (OtherBodyIndex :type Integer) (bFromSweep :type Boolean) (SweepResult :type "HitResult Structure (by ref)"))
  (`self.CeintureServeurEquip` OtherActor))

(event `self.Box.OnComponentEndOverlap`
  (params (OverlappedComponent :type "PrimitiveComponent Object Reference") (OtherActor :type "Actor Object Reference") (OtherComp :type "PrimitiveComponent Object Reference") (OtherBodyIndex :type Integer)))

(event `self.Sphere.OnComponentBeginOverlap`
  (params (OverlappedComponent :type "PrimitiveComponent Object Reference") (OtherActor :type "Actor Object Reference") (OtherComp :type "PrimitiveComponent Object Reference") (OtherBodyIndex :type Integer) (bFromSweep :type Boolean) (SweepResult :type "HitResult Structure (by ref)")))

(event `self.Sphere.OnComponentEndOverlap`
  (params (OverlappedComponent :type "PrimitiveComponent Object Reference") (OtherActor :type "Actor Object Reference") (OtherComp :type "PrimitiveComponent Object Reference") (OtherBodyIndex :type Integer)))

(fn `UserConstructionScript`)